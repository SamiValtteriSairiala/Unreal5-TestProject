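; Base enemy Blueprint that shows a world health bar and takes damage from projectile hits.
; On BeginPlay it makes itself the owner of the EnemyHealthBar widget in its HealthBar component.
; Every Tick it re-casts that widget and toggles its visibility from the IsSeen flag.
; Hits from FPSTestProjectile actors call TakeDamage with a fixed small amount.
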(event `self.ReceiveBeginPlay`
  (bind _asenemy_health_bar (cast `/Game/EnemyHealthBar` (`WidgetComponent.GetUserWidgetObject` (`self.HealthBar`))))
  (set `/Game/EnemyHealthBar.HealthBarOwner` self _asenemy_health_bar))

(event `self.ReceiveTick`
  (params (DeltaSeconds :type "Float (single-precision)"))
  (if (`self.isSeen`)
    (bind _asenemy_health_bar (cast `/Game/EnemyHealthBar` (`WidgetComponent.GetUserWidgetObject` (`self.HealthBar`))))
    (set `/Game/EnemyHealthBar.HealthBarOwner` self _asenemy_health_bar)
    (`Widget.SetVisibility` _asenemy_health_bar "Visible")
    (else
      (bind _asenemy_health_bar_2 (cast `/Game/EnemyHealthBar` (`WidgetComponent.GetUserWidgetObject` (`self.HealthBar`))))
      (`Widget.SetVisibility` _asenemy_health_bar_2 "Hidden"))))

(event `self.ReceiveHit`
  (params (MyComp :type "PrimitiveComponent Object Reference") (Other :type "Actor Object Reference") (OtherComp :type "PrimitiveComponent Object Reference") (bSelfMoved :type Boolean) (HitLocation :type "Vector Structure") (HitNormal :type "Vector Structure") (NormalImpulse :type "Vector Structure") (Hit :type "HitResult Structure (by ref)"))
  (cast `FPSTestProjectile` Other)
  (`self.TakeDamage` 0.1))

(fn `UserConstructionScript`)